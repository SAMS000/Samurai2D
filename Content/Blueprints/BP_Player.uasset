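; BP_Player is a Paper2D player Blueprint with a flipbook sprite and a Space-triggered melee attack.
; Space switches the sprite to the non-looping Attack1 flipbook and sets IsAttacking, which makes Tick run HitCheck and unhide HitBox.
; HitCheck loops over overlapping PaperSpriteActors, but its ApplyDamage is unconnected.
; The idle reset and Attack1 call are also unconnected, so IsAttacking is never cleared.
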(event `Key|SpaceBar`
  (params (Key :type "Key Structure"))
  (bind _sprite (`self.Sprite`))
  ;[1 1 1] Attack1
  (:`Pressed`
    (`PaperFlipbookComponent.SetFlipbook` _sprite "/Game/SamuraiAssets/RedSamurai/Spritesheet/sheets/Attack1.Attack1")
    (`PaperFlipbookComponent.SetLooping` _sprite false)
    (set `self.IsAttacking` true)))

(event `self.ReceiveTick`
  (params (DeltaSeconds :type "Float (single-precision)"))
  (if (`self.IsAttacking`)
    (`self.HitCheck`)
    (`SceneComponent.SetHiddenInGame` (`self.HitBox`) false false)))

(fn `Attack1`
  (bind _sprite (`self.Sprite`))
  (`PaperFlipbookComponent.SetFlipbook` _sprite "/Game/SamuraiAssets/RedSamurai/Spritesheet/sheets/Attack1.Attack1")
  (`PaperFlipbookComponent.SetLooping` _sprite false)
  (if (not (`PaperFlipbookComponent.IsPlaying` _sprite))
    (`PaperFlipbookComponent.Play` _sprite)))

(fn `HitCheck`
  (for _array_element (`PrimitiveComponent.GetOverlappingActors` (`self.HitBox`) "/Script/Paper2D.PaperSpriteActor")
    (if (!= _array_element self)
      _)))

(fn `UserConstructionScript`)